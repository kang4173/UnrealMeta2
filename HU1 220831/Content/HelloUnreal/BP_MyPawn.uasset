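; BP_MyPawn is an input-practice pawn that flies relative to the camera and prints debug output for test axis and action mappings.
; Movement axes offset the actor along camera forward and right by Speed, without sweep or delta-time scaling, while look axes add controller pitch and yaw.
; SpeedUp and SpeedDown step Speed within clamped limits and print it.
; A minutes-and-seconds elapsed-time printer (PrintTime, IntToStr00) exists but is disconnected from Tick.
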(event `self.ReceiveBeginPlay`)

(event `self.ReceiveTick`
  (params (DeltaSeconds :type "Float (single-precision)")))

(event `InputAxis|AxisTest`
  (params (AxisValue :type "Float (single-precision)"))
  ;[1 1 1] 축매핑 테스트
  (`KismetSystemLibrary.PrintString` (`KismetStringLibrary.Concat_StrStr` "" (`KismetStringLibrary.Conv_DoubleToString` AxisValue))))

(event `InputAction|TestKey`
  (params (Key :type "Key Structure"))
  ;[1 1 1] 액션매핑 테스트
  (:`Pressed`
    (`KismetSystemLibrary.PrintString` "Pressed"))
  (:`Released`
    (`KismetSystemLibrary.PrintString` "Released")))

(event `InputAxis|MoveForward`
  (params (AxisValue :type "Float (single-precision)"))
  ;[1 1 1] Move
  (`self.K2_AddActorWorldOffset` (* (`self.GetActorForwardVector` (`GameplayStatics.GetPlayerCameraManager` 0)) (* AxisValue (`self.Speed`)))))

(event `InputAction|SpeedUp`
  (params (Key :type "Key Structure"))
  ;[1 1 1] 10~100 , 10증감.
  (:`Pressed`
    (bind _output_get (set `self.Speed` (`KismetMathLibrary.FClamp` (+ (`self.Speed`) 10.0) 10.0 100.0)))
    (`KismetSystemLibrary.PrintString` (`KismetStringLibrary.Concat_StrStr` "Speed" (`KismetStringLibrary.Conv_DoubleToString` _output_get)))))

(event `InputAxis|MoveRight`
  (params (AxisValue :type "Float (single-precision)"))
  ;[1 1 1] Move
  (`self.K2_AddActorWorldOffset` (* (`self.GetActorRightVector` (`GameplayStatics.GetPlayerCameraManager` 0)) (* AxisValue (`self.Speed`)))))

(event `InputAction|SpeedDown`
  (params (Key :type "Key Structure"))
  ;[1 1 1] 10~100 , 10증감.
  (:`Pressed`
    (bind _output_get (set `self.Speed` (`KismetMathLibrary.FClamp` (- (`self.Speed`) 10.0) 10.0 100.0)))
    (`KismetSystemLibrary.PrintString` (`KismetStringLibrary.Concat_StrStr` "Speed" (`KismetStringLibrary.Conv_DoubleToString` _output_get)))))

(event `InputAxis|LookUp`
  (params (AxisValue :type "Float (single-precision)"))
  ;[1 1 1] 카메라회전?
  (`self.AddControllerPitchInput` AxisValue))

(event `InputAxis|LookRight`
  (params (AxisValue :type "Float (single-precision)"))
  ;[1 1 1] 카메라회전?
  (`self.AddControllerYawInput` AxisValue))

(fn `IntToStr00`
  (params (Number :type "Float (double-precision)"))
  (returns (Sring :type String))
  (bind _returnvalue (`KismetMathLibrary.FFloor` Number))
  (bind _returnvalue_2 (`KismetStringLibrary.Conv_IntToString` _returnvalue))
  (if (< _returnvalue 10)
    (return (`KismetStringLibrary.Concat_StrStr` "0" _returnvalue_2))
    (else
      (return _returnvalue_2))))

(fn `PrintTime`
  (params (DeltaSeconds :type "Float (double-precision)"))
  (bind _output_get (set `self.Total Delta Seconds` (+ (`self.Total Delta Seconds`) DeltaSeconds)))
  (bind _sring (`self.IntToStr00` (/ _output_get 60.0)))
  (bind _sring_2 (`self.IntToStr00` (mod _output_get 60.0)))
  (bind _returnvalue (`KismetStringLibrary.Concat_StrStr` _sring "분" _sring_2 "초"))
  (if (`KismetStringLibrary.NotEqual_StrStr` _returnvalue (`self.BeforeString`))
    (`KismetSystemLibrary.PrintString` _returnvalue)
    (set `self.BeforeString` _returnvalue)))

(fn `UserConstructionScript`)