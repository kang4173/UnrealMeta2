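; BP_MyPawn is a pawn that works as an on-screen play timer, printing elapsed minutes and seconds with Korean unit labels.
; Tick feeds delta time into PrintTime, which accumulates it and builds the label using IntToStr00 to floor and zero-pad each number.
; It caches the last string so it prints only when the displayed time changes.
; The BeginPlay name print has both screen and log output disabled.
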(event `self.ReceiveBeginPlay`
  (`KismetSystemLibrary.PrintString` (`KismetSystemLibrary.GetDisplayName` self) false false (struct :`G` 0.66 :`B` 1.0 :`A` 1.0) 60.0))

(event `self.ReceiveTick`
  (params (DeltaSeconds :type "Float (single-precision)"))
  ;[1 1 1] DeltaSeconds
  (`self.PrintTime` (* DeltaSeconds 1.0)))

(fn `IntToStr00`
  (params (Number :type "Float (double-precision)"))
  (returns (Sring :type String))
  (bind _returnvalue (`KismetMathLibrary.FFloor` Number))
  (bind _returnvalue_2 (`KismetStringLibrary.Conv_IntToString` _returnvalue))
  (if (< _returnvalue 10)
    (return (`KismetStringLibrary.Concat_StrStr` "0" _returnvalue_2))
    (else
      (return _returnvalue_2))))

(fn `PrintTime`
  (params (DeltaSeconds :type "Float (double-precision)"))
  (bind _output_get (set `self.Total Delta Seconds` (+ (`self.Total Delta Seconds`) DeltaSeconds)))
  (bind _sring (`self.IntToStr00` (/ _output_get 60.0)))
  (bind _sring_2 (`self.IntToStr00` (mod _output_get 60.0)))
  (bind _returnvalue (`KismetStringLibrary.Concat_StrStr` _sring "분" _sring_2 "초"))
  (if (`KismetStringLibrary.NotEqual_StrStr` _returnvalue (`self.BeforeString`))
    (`KismetSystemLibrary.PrintString` _returnvalue)
    (set `self.BeforeString` _returnvalue)))

(fn `UserConstructionScript`)