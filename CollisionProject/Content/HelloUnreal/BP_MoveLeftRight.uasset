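; Actor Blueprint that slides its StaticMesh back and forth along its relative X axis.
; The custom event yyyy plays or reverses a timeline based on IsMoveRight, scaling its value into the mesh's X location.
; When the timeline finishes, it flips the flag and loops back to the branch for continuous ping-pong motion.
; BeginPlay is empty, nothing here calls yyyy, and the input-enable and timeline debug-print nodes are disconnected.
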(event `Key|B`
  (params (Key :type "Key Structure")))

(event `yyyy`
  (if (`self.IsMoveRight`) :!label _label
    (bind (_direction _value) (`Timeline|타임라인_0` :!label _label_2)
      (:`Update`
        (`SceneComponent.K2_SetRelativeLocation` (`self.StaticMesh`) (`KismetMathLibrary.MakeVector` (* 1000.0 _value)) false false))
      (:`Finished`
        (set `self.IsMoveRight` (not (`self.IsMoveRight`)))
        (goto _label)))
    (else
      (goto _label_2 :!via `Reverse`))))

(event `self.ReceiveBeginPlay`)

(fn `UserConstructionScript`)