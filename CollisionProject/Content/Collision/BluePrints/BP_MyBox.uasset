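; BP_MyBox is a collision test Blueprint that reports what touches its Cube2 component.
; Begin overlap, end overlap and hit events each print the display names of the component, other actor and other component as long-lasting screen messages.
; The remaining graph holds disconnected practice nodes for sequences, loops and playing MoveRect, RocationBall and MoveLeftRight, none of which run.
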(event `self.ReceiveBeginPlay`)

(event `self.Cube2.OnComponentBeginOverlap`
  (params (OverlappedComponent :type "PrimitiveComponent Object Reference") (OtherActor :type "Actor Object Reference") (OtherComp :type "PrimitiveComponent Object Reference") (OtherBodyIndex :type Integer) (bFromSweep :type Boolean) (SweepResult :type "HitResult Structure (by ref)"))
  ;[1 1 1] Begin overlapped
  (`KismetSystemLibrary.PrintString` (`KismetStringLibrary.Concat_StrStr` "Begin Overlapped Component" (`KismetSystemLibrary.GetDisplayName` OverlappedComponent) "Other Actor" (`KismetSystemLibrary.GetDisplayName` OtherActor) "Other Comp" (`KismetSystemLibrary.GetDisplayName` OtherComp)) true true (struct :`G` 0.66 :`B` 1.0 :`A` 1.0) 200.0))

(event `self.RocationBall.OnInputTouchBegin`
  (params (FingerIndex :type "ETouchIndex Enum" :default "Touch1") (TouchedActor :type "Actor Object Reference")))

(event `self.Cube2.OnComponentEndOverlap`
  (params (OverlappedComponent :type "PrimitiveComponent Object Reference") (OtherActor :type "Actor Object Reference") (OtherComp :type "PrimitiveComponent Object Reference") (OtherBodyIndex :type Integer))
  ;[1 1 1] End Overlapped
  (`KismetSystemLibrary.PrintString` (`KismetStringLibrary.Concat_StrStr` "End Overlapped Component" (`KismetSystemLibrary.GetDisplayName` OverlappedComponent) "Other Actor" (`KismetSystemLibrary.GetDisplayName` OtherActor) "Other Comp" (`KismetSystemLibrary.GetDisplayName` OtherComp)) true true (struct :`G` 0.66 :`B` 1.0 :`A` 1.0) 200.0))

(event `self.Cube2.OnComponentHit`
  (params (HitComponent :type "PrimitiveComponent Object Reference") (OtherActor :type "Actor Object Reference") (OtherComp :type "PrimitiveComponent Object Reference") (NormalImpulse :type "Vector Structure") (Hit :type "HitResult Structure (by ref)"))
  ;[1 1 1] Hit
  (`KismetSystemLibrary.PrintString` (`KismetStringLibrary.Concat_StrStr` "Hit Overlapped Component" (`KismetSystemLibrary.GetDisplayName` HitComponent) "Other Actor" (`KismetSystemLibrary.GetDisplayName` OtherActor) "Other Comp" (`KismetSystemLibrary.GetDisplayName` OtherComp)) true true (struct :`G` 0.66 :`B` 1.0 :`A` 1.0) 200.0))

(fn `UserConstructionScript`)